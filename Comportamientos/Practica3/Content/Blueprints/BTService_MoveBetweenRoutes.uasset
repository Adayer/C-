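; Behavior Tree service that cycles an AI character through its Waypoints route by updating the blackboard.
; While active, it binds to the AIControllerBP's ReceiveMoveCompleted event and unbinds on deactivation.
; Each successful move increments RouteIndex with wraparound, then sets WaypointLocation from that actor array.
; The location lookup recomputes index + 1 after the write, so it points one waypoint past the stored RouteIndex.
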(event `self.ReceiveDeactivation`
  (params (OwnerActor :type "Actor Object Reference"))
  (bind _asaicontroller_bp (cast `/Game/Blueprints/AIControllerBP` OwnerActor))
  (remove `AIController.ReceiveMoveCompleted` _asaicontroller_bp (delegate `ReceiveMoveCompleted_Event_0`)))

(event `self.ReceiveActivation`
  (params (OwnerActor :type "Actor Object Reference"))
  (bind _asaicontroller_bp (cast `/Game/Blueprints/AIControllerBP` OwnerActor))
  (bind _output_get (set `self.AICntrlRef` _asaicontroller_bp))
  (add `AIController.ReceiveMoveCompleted` _output_get (delegate `ReceiveMoveCompleted_Event_0`)))

(event `ReceiveMoveCompleted_Event_0`
  (params (RequestID :type "AIRequestID Structure") (Result :type "EPathFollowingResult Enum" :default "Success"))
  (switch `EPathFollowingResult` Result
    (:`Success`
      (bind _asaicharacter_bp (cast `/Game/Blueprints/AICharacterBP` (`Controller.K2_GetPawn` (`self.AICntrlRef`))))
      (bind _waypoints (`/Game/Blueprints/AICharacterBP.Waypoints` _asaicharacter_bp))
      (bind _returnvalue (mod (+ (`BTFunctionLibrary.GetBlackboardValueAsInt` (`self.RouteIndex`)) 1) (`KismetArrayLibrary.Array_Length` _waypoints)))
      (`BTFunctionLibrary.SetBlackboardValueAsInt` (`self.RouteIndex`) _returnvalue)
      (`BTFunctionLibrary.SetBlackboardValueAsVector` (`self.WaypointLocation`) (`Actor.K2_GetActorLocation` (`|GetArrayItem` _waypoints _returnvalue))))))