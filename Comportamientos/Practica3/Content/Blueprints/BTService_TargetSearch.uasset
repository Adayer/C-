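; Behavior Tree service that finds a visible target for an AI-controlled pawn and writes it to the Blackboard.
; Each tick, a sphere trace around the pawn gathers nearby objects of the desired types, ignoring all AICharacterBP actors.
; Camera-channel line traces check line of sight, and the first visible hit sets TargetToFollow and TargetLocation.
; Blocked candidates clear TargetToFollow but leave TargetLocation untouched; an empty sweep changes neither key.
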(event `self.ReceiveTickAI`
  (params (OwnerController :type "AIController Object Reference") (ControlledPawn :type "Pawn Object Reference") (DeltaSeconds :type "Float (single-precision)"))
  (if (not (`KismetSystemLibrary.IsValid` (`self.AICtrlRef`)))
    (bind _asaicontroller_bp (cast `/Game/Blueprints/AIControllerBP` OwnerController))
    (set `self.AICtrlRef` _asaicontroller_bp))
  (bind _output_get (set `self.MyLocation` (`Actor.K2_GetActorLocation` (`Controller.K2_GetPawn` (`self.AICtrlRef`)))))
  (bind _outactors (`GameplayStatics.GetAllActorsOfClass` "/Game/Blueprints/AICharacterBP.AICharacterBP_C"))
  (bind _outhits (`KismetSystemLibrary.SphereTraceMultiForObjects` _output_get (+ _output_get (0.0 0.0 15.0)) 1500.0 (`self.DesiredObjectTypes`) false _outactors))
  (for _array_element _outhits
    (bind (_bblockinghit _binitialoverlap _time _distance _location _impactpoint _normal _impactnormal _physmat _hitactor) (`GameplayStatics.BreakHitResult` _array_element))
    (bind _outhit (`KismetSystemLibrary.LineTraceSingle` (`self.MyLocation`) (`Actor.K2_GetActorLocation` _hitactor) "TraceTypeQuery2" false _outactors))
    (bind (_bblockinghit_2 _binitialoverlap_2 _time_2 _distance_2 _location_2 _impactpoint_2 _normal_2 _impactnormal_2 _physmat_2 _hitactor_2) (`GameplayStatics.BreakHitResult` _outhit))
    (if (== _hitactor_2 _hitactor)
      (`BTFunctionLibrary.SetBlackboardValueAsObject` (`self.TargetToFollow`) _hitactor_2)
      (`BTFunctionLibrary.SetBlackboardValueAsVector` (`self.TargetLocation`) (`Actor.K2_GetActorLocation` _hitactor_2))
      (break)
      (else
        (`BTFunctionLibrary.SetBlackboardValueAsObject` (`self.TargetToFollow`))))))