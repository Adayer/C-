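; Behavior tree decorator that checks whether an AI pawn is within an acceptable distance of its follow target.
; The owner is cast to AIControllerBP, and the check fails if that cast does not succeed.
; It passes when the distance from the controlled pawn to the TargetToFollow blackboard actor is at most AcceptableDistance.
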(fn `PerformConditionCheck`
  (params (OwnerActor :type "Actor Object Reference"))
  (returns (ReturnValue :type Boolean))
  (bind _asaicontroller_bp (cast `/Game/Blueprints/AIControllerBP` OwnerActor)
    (:`then`
      (bind _output_get (set `self.AICtrlRef` _asaicontroller_bp))
      (return (>= (`self.AcceptableDistance`) (`KismetMathLibrary.VSize` (- (`Actor.K2_GetActorLocation` (`Controller.K2_GetPawn` _output_get)) (`Actor.K2_GetActorLocation` (`BTFunctionLibrary.GetBlackboardValueAsActor` (`self.TargetToFollow`))))))))
    (:`CastFailed`
      (return false))))