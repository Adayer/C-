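; AI controller that patrols its pawn between WaypointBP actors and chases actors it perceives.
; An integer State switches patrol and chase; move-completed callbacks advance the waypoint loop or re-issue moves toward perceived actors beyond close range.
; Successful sensing stops movement, so the aborted move starts the chase; lost sensing resumes patrol at the nearest waypoint.
; Tick draws two debug radius spheres around the pawn.
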(event `self.ReceiveBeginPlay`
  (`self.SetPatrol`)
  (`self.SetStateMachine`))

(event `SetPatrol`
  (bind _outactors (`GameplayStatics.GetAllActorsOfClass` "/Game/Blueprints/WaypointBP.WaypointBP_C"))
  (bind _output_get (set `self.Waypoints` _outactors))
  (bind _output_get_2 (set `self.Index` 0))
  (set `self.CurrentWaypoint` (`|GetArrayItem` _output_get _output_get_2))
  (add `self.ReceiveMoveCompleted` (delegate `OnArriveAtWaypoint`))
  (`self.MoveToActor` (`self.CurrentWaypoint`) -1.0 true true true null))

(event `OnArriveAtWaypoint` :!signature `self.ReceiveMoveCompleted`
  (params (RequestID :type "AIRequestID Structure") (Result :type "EPathFollowingResult Enum" :default "Success"))
  (switch `EPathFollowingResult` Result
    (:`Success`
      _)
    (:`Aborted`
      _))
  (if (== (`self.State`) 0)
    (`KismetSystemLibrary.RetriggerableDelay` 0.5)
    (set `self.Index` (mod (+ (`self.Index`) 1) (`KismetArrayLibrary.Array_Length` (`self.Waypoints`))))
    (bind _output_get (set `self.CurrentWaypoint` (`|GetArrayItem` (`self.Waypoints`) (`self.Index`))))
    (`self.MoveToActor` _output_get -1.0 true true true null)
    (elif (== (`self.State`) 1)
      (for _array_element (stale `self.PerceptionUpdated` UpdatedActors)
        (if (<= (`KismetMathLibrary.VSize` (- (`self.K2_GetActorLocation` _array_element) (`self.K2_GetActorLocation` (`self.K2_GetPawn`)))) 100.0)
          (break)
          (else
            (`self.MoveToActor` _array_element -1.0 true true true null)))))))

(event `SetStateMachine`
  (set `self.State` 0))

(event `self.PerceptionUpdated`
  (params (UpdatedActors :type "Array of Actor Object Reference (by ref)"))
  (`self.CheckStimuli` UpdatedActors))

(event `self.ReceiveTick`
  (params (DeltaSeconds :type "Float (single-precision)"))
  (bind _returnvalue (`self.K2_GetActorLocation` (`self.K2_GetPawn`)))
  (`KismetSystemLibrary.DrawDebugSphere` _returnvalue 1000.0 12 (struct :`R` 0.342294 :`G` 1.0 :`A` 1.0) 0.1 1.0)
  (`KismetSystemLibrary.DrawDebugSphere` _returnvalue 750.0 12 (struct :`R` 1.0 :`B` 0.00868 :`A` 1.0) 0.1 1.0))

(event `CheckStimuli`
  (params (NewParam :type "Array of Actor Object Reference"))
  (`KismetSystemLibrary.PrintString` (`KismetStringLibrary.Conv_IntToString` (`KismetArrayLibrary.Array_Length` NewParam)))
  (for _array_element NewParam
    (bind _info (`AIPerceptionComponent.GetActorsPerception` (`self.PerceptionCmp`) _array_element))
    (if (`.bSuccessfullySensed` (break `AIStimulus` (`|GetArrayItem` (`.LastSensedStimuli` (break `ActorPerceptionBlueprintInfo` _info)))))
      (if (== (`self.State`) 0)
        (if (>= (`KismetArrayLibrary.Array_Length` NewParam) 1)
          (set `self.State` 1)
          (`self.StopMovement`)))
      (else
        (set `self.State` 0)
        (set `self.BufferBestDistance` 10000000.0)
        (for (_array_element_2 _array_index) (`self.Waypoints`)
          (bind _returnvalue (`KismetMathLibrary.VSize` (- (`self.K2_GetActorLocation` (`self.K2_GetPawn`)) (`self.K2_GetActorLocation` _array_element_2))))
          (if (< _returnvalue (`self.BufferBestDistance`))
            (set `self.BufferBestDistance` _returnvalue)
            (set `self.Index` _array_index)))
        (`self.MoveToActor` (`|GetArrayItem` (`self.Waypoints`) (`self.Index`)) -1.0 true true true null)))))

(fn `UserConstructionScript`)