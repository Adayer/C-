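; AI controller that keeps a soldier pawn wandering between waypoints assigned to it.
; It gathers unlocked WaypointBP actors that list the controlled AISoldierBP, shuffles them, locks the first and issues a move.
; When the move completes, it pauses briefly, unlocks that waypoint and picks again.
; The lock acts as a reservation so other soldiers skip occupied waypoints, with no guard for an empty candidate list.
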(event `self.ReceiveBeginPlay`
  (bind _posiblewaypoints (`self.PosibleWaypoints`))
  (add `self.ReceiveMoveCompleted` (delegate `ChooseDestination`))
  (`KismetArrayLibrary.Array_Clear` (`self.PosibleWaypoints`) :!label _label)
  (bind _outactors (`GameplayStatics.GetAllActorsOfClass` "/Game/Blueprints/WaypointBP.WaypointBP_C"))
  (for _array_element _outactors
    (bind _asaisoldier_bp (cast `/Game/Blueprints/AISoldierBP` (`self.K2_GetPawn`)))
    (if (and (!= (`KismetArrayLibrary.Array_Find` (`/Game/Blueprints/WaypointBP.AI_Characters` _array_element) _asaisoldier_bp) -1) (not (`/Game/Blueprints/WaypointBP.Locked` _array_element)))
      (`KismetArrayLibrary.Array_Add` (`self.PosibleWaypoints`) _array_element)))
  (`KismetArrayLibrary.Array_Shuffle` _posiblewaypoints)
  (set `/Game/Blueprints/WaypointBP.Locked` true (`|GetArrayItem` _posiblewaypoints))
  (`self.MoveToActor` null -1.0 true true true null))

(event `ChooseDestination` :!signature `self.ReceiveMoveCompleted`
  (params (RequestID :type "AIRequestID Structure") (Result :type "EPathFollowingResult Enum" :default "Success"))
  (`KismetSystemLibrary.Delay` 3.0)
  (set `/Game/Blueprints/WaypointBP.Locked` false (`|GetArrayItem` (`self.PosibleWaypoints`)))
  (goto _label))

(fn `UserConstructionScript`)