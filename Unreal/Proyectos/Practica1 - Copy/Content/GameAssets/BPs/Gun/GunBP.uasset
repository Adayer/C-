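; GunBP is a player-controlled gun actor that fires from its arrow's transform and can hop between preset locations.
; On BeginPlay it enables input from player 0 and moves its root to the current entry in an array of location actors.
; Fire passes the arrow transform to GunComponent, while the C key moves the gun to the next location, wrapping around.
; DoOnce gates limit both actions to once per press.
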(event `self.ReceiveBeginPlay`
  (`self.EnableInput` (`GameplayStatics.GetPlayerController` 0))
  (`SceneComponent.K2_SetWorldLocation` (`self.DefaultSceneRoot`) (`self.K2_GetActorLocation` (`|GetArrayItem` (`self.Locations`) (`self.Index`))) false false)
  (set `self.Index` (mod (+ (`self.Index`) 1) (`KismetArrayLibrary.Array_Length` (`self.Locations`)))))

(event `InputAction|Fire`
  (params (Key :type "Key Structure"))
  (:`Pressed`
    (`/Engine/EditorBlueprintResources/StandardMacros.DoOnce` false :!label _label
      (:`Completed`
        (`/Game/GameAssets/BPs/Components/GunComponent.TriggerPressed` (`self.GunComponent`) (`SceneComponent.K2_GetComponentToWorld` (`self.Arrow`))))))
  (:`Released`
    (goto _label :!via `Reset`)))

(event `Key|C`
  (params (Key :type "Key Structure"))
  (:`Pressed`
    (`/Engine/EditorBlueprintResources/StandardMacros.DoOnce` false :!label _label_2
      (:`Completed`
        (`SceneComponent.K2_SetWorldLocation` (`self.DefaultSceneRoot`) (`self.K2_GetActorLocation` (`|GetArrayItem` (`self.Locations`) (`self.Index`))) false false)
        (set `self.Index` (mod (+ (`self.Index`) 1) (`KismetArrayLibrary.Array_Length` (`self.Locations`)))))))
  (:`Released`
    (goto _label_2 :!via `Reset`)))

(fn `UserConstructionScript`)