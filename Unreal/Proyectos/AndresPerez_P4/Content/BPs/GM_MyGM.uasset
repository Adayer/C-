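; GM_MyGM is a game mode that runs a timed level and awards points for obstacle hits.
; On BeginPlay, one timer calls NextLevel after the level time, while a looping timer decrements CurrentTimer every tenth of a second for UI display.
; NextLevel and ObstacleHit forward to GI_MyGameInstance, which handles level progression and adds the per-obstacle points.
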(event `self.ReceiveBeginPlay`
  (`KismetSystemLibrary.K2_SetTimerDelegate` (delegate `NextLevel`) (`self.Timer`))
  ;[1 1 1] UI
  (set `self.CurrentTimer` (`self.Timer`))
  (`KismetSystemLibrary.K2_SetTimerDelegate` (delegate `UpdateTimer`) 0.1 true))

(event `UpdateTimer`
  ;[1 1 1] UI
  (set `self.CurrentTimer` (- (`self.CurrentTimer`) 0.1)))

(event `NextLevel`
  (bind _asgi_my_game_instance (cast `/Game/BPs/GI_MyGameInstance` (`GameplayStatics.GetGameInstance`)))
  (`/Game/BPs/GI_MyGameInstance.NextLevel` _asgi_my_game_instance))

(event `ObstacleHit`
  (bind _asgi_my_game_instance (cast `/Game/BPs/GI_MyGameInstance` (`GameplayStatics.GetGameInstance`)))
  (`/Game/BPs/GI_MyGameInstance.AddPoints` _asgi_my_game_instance (`self.PointsPerObstacle`)))

(fn `UserConstructionScript`)