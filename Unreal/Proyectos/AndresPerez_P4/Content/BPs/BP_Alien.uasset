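; BP_Alien is an alien that moves in response to player axis input.
; The ForwardInput and RightInput axis events scale the collision component's forward and right vectors by the axis value.
; Each result goes to the movement component as a non-forced input vector, so movement is relative to the collision component's facing.
; The construction script is empty.
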(event `InputAxis|ForwardInput`
  (params (AxisValue :type "Float (single-precision)"))
  (`PawnMovementComponent.AddInputVector` (`self.MovementComponent`) (* (`SceneComponent.GetForwardVector` (`self.CollisionComponent`)) AxisValue) false))

(event `InputAxis|RightInput`
  (params (AxisValue :type "Float (single-precision)"))
  (`PawnMovementComponent.AddInputVector` (`self.MovementComponent`) (* (`SceneComponent.GetRightVector` (`self.CollisionComponent`)) AxisValue) false))

(fn `UserConstructionScript`)